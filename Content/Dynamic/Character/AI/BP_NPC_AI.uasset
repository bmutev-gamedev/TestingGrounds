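; AI controller for guard NPCs that runs the GuardBehaviour tree on the PatrolData blackboard from BeginPlay.
; Perception updates write any sensed actor without the "Friendly" tag to the enemy blackboard key, and clear the key when such an actor is no longer sensed.
; A LogPerceptionInfo helper prints pawn, perception type and detected actor, but nothing here calls it.
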(event `self.ReceiveBeginPlay`
  (bind _blackboardcomponent (`self.UseBlackboard` "/Game/Dynamic/Character/AI/PatrolData.PatrolData"))
  (set `self.BlackboardComp` _blackboardcomponent)
  (`self.RunBehaviorTree` "/Game/Dynamic/Character/AI/GuardBehaviour.GuardBehaviour"))

(event `self.AIPerception.OnTargetPerceptionUpdated`
  (params (Actor :type "Actor Object Reference") (Stimulus :type "AIStimulus Structure"))
  (`self.Update Blackboard EnemyKey` Actor Stimulus))

(fn `Update Blackboard EnemyKey`
  (params (Actor :type "Actor Object Reference") (Stimulus :type "AIStimulus Structure"))
  (`/Engine/EditorBlueprintResources/StandardMacros.IsValid` Actor
    (:`Is Valid`
      (if (`self.ActorHasTag` Actor "Friendly")
        _
        (elif (`.bSuccessfullySensed` (break `AIStimulus` Stimulus))
          (`BlackboardComponent.SetValueAsObject` (`self.BlackboardComp`) (`self.EnemyKey`) Actor)
          (else
            (`BlackboardComponent.ClearValue` (`self.BlackboardComp`) (`self.EnemyKey`))))))))

(fn `UserConstructionScript`)