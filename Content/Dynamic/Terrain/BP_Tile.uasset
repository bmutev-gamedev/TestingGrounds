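; Terrain tile for an endless level that scatters props and gates the player's progress with a barrier.
; On BeginPlay it locks the barrier and calls PlaceActors per prop type with count, radius and, for rocks, scale limits.
; The player entering BarrierTrigger unlocks it; leaving relocks it and asks InfiniteTerrainGameMode to spawn another tile.
; TileDestructionTrigger destroys the tile on player overlap, and GetAttachLocation exposes the Arrow transform.
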(event `self.ReceiveBeginPlay`
  (`self.Lock`)
  (`self.PlaceActors` "/Game/Static/TestingGroundPack/IndustryPropsPack4/Blueprints/BP_Container.BP_Container_C" 1 2 400.0)
  (`self.PlaceActors` "/Game/Static/TestingGroundPack/IndustryPropsPack4/Blueprints/BP_Crate.BP_Crate_C" 1 2 150.0)
  (`self.PlaceActors` "/Game/Static/TestingGroundPack/IndustryPropsPack4/Blueprints/BP_Canisters.BP_Canisters_C" 1 3 70.0)
  (`self.PlaceActors` "/Game/Static/TestingGroundPack/RockPackProV1/Blueprints/BP_Rock1.BP_Rock1_C" 0 3 150.0 1.0 5.0)
  (`self.PlaceActors` "/Game/Static/TestingGroundPack/RockPackProV1/Blueprints/BP_Rock2.BP_Rock2_C" 0 2 250.0 1.0 5.0)
  (`self.PlaceActors` "/Game/Static/TestingGroundPack/RockPackProV1/Blueprints/BP_Rock3.BP_Rock3_C" 0 2 250.0 1.0 5.0)
  (`self.PlaceActors` "/Game/Static/TestingGroundPack/IndustryPropsPack4/Blueprints/BP_Sandbags.BP_Sandbags_C" 0 2 250.0))

(event `self.BarrierTrigger.OnComponentBeginOverlap`
  (params (OverlappedComponent :type "PrimitiveComponent Object Reference") (OtherActor :type "Actor Object Reference") (OtherComp :type "PrimitiveComponent Object Reference") (OtherBodyIndex :type Integer) (bFromSweep :type Boolean) (SweepResult :type "HitResult Structure (by ref)"))
  (`self.IsPlayerActor` OtherActor
    (:`true`
      (`self.Unlock`))))

(event `self.BarrierTrigger.OnComponentEndOverlap`
  (params (OverlappedComponent :type "PrimitiveComponent Object Reference") (OtherActor :type "Actor Object Reference") (OtherComp :type "PrimitiveComponent Object Reference") (OtherBodyIndex :type Integer))
  (`self.IsPlayerActor` OtherActor
    (:`true`
      (`self.Lock`)
      (bind _asinfinite_terrain_game_mode (cast `/Game/Dynamic/InfiniteTerrainGameMode` (`GameplayStatics.GetGameMode`)))
      (`/Game/Dynamic/InfiniteTerrainGameMode.SpawnTile` _asinfinite_terrain_game_mode))))

(event `self.TileDestructionTrigger.OnComponentBeginOverlap`
  (params (OverlappedComponent :type "PrimitiveComponent Object Reference") (OtherActor :type "Actor Object Reference") (OtherComp :type "PrimitiveComponent Object Reference") (OtherBodyIndex :type Integer) (bFromSweep :type Boolean) (SweepResult :type "HitResult Structure (by ref)"))
  (`self.IsPlayerActor` OtherActor
    (:`true`
      (`self.K2_DestroyActor`))))

(fn `GetAttachLocation`
  (returns (AttachtTransform :type "Transform Structure"))
  (return (`SceneComponent.K2_GetComponentToWorld` (`self.Arrow`))))

(fn `Lock`
  (`PrimitiveComponent.SetCollisionEnabled` (`self.Barrier`) "QueryAndPhysics")
  (`PrimitiveComponent.SetMaterial` (`self.Barrier`) 0 "/Game/Dynamic/Terrain/MI_Barrier_Red.MI_Barrier_Red"))

(fn `Unlock`
  (`PrimitiveComponent.SetCollisionEnabled` (`self.Barrier`) "NoCollision")
  (`PrimitiveComponent.SetMaterial` (`self.Barrier`) 0 "/Game/Dynamic/Terrain/MI_Barrier_Green.MI_Barrier_Green")
  (return))

(fn `UserConstructionScript`)